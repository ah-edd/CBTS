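; BP_Oven is a configurable kitchen oven prop, assembled entirely in the Construction Script from hierarchical instanced static mesh components.
; It adds one instance each for body, door, grille, five knobs and hobs, with exposed values setting door roll, grille height and knob pitch.
; Toggles add an optional tray that follows the grille height, a countertop and four burner flames.
; The Event Graph has no runtime logic.
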(event EventBeginPlay)

(event Collision|EventActorBeginOverlap
  (params (OtherActor :type Actor%20Object%20Reference)))

(event EventTick
  (params (DeltaSeconds :type Float%20%28single-precision%29)))

(fn ConstructionScript
  (Utilities|FlowControl|Sequence
    (:then_0
      (Components|InstancedStaticMesh|AddInstance (Variables|Default|GetHISM_OvenMain) (Math|Transform|MakeTransform "0, 0, 0" "0, 0, 0" "1,1,1"))
      (Components|InstancedStaticMesh|AddInstance (Variables|Default|GetHISM_OvenDoor) (Math|Transform|MakeTransform "37.500000,46.000000,21.000000" (Math|Rotator|MakeRotator (Variables|Default|GetOpen%20Door) 0.0 0.0) "1,1,1"))
      (Components|InstancedStaticMesh|AddInstance (Variables|Default|GetHISM_OvenGrille) (Math|Transform|MakeTransform (Math|Vector|MakeVector 0.0 0.0 (Variables|Default|GetAdjust%20Grille)) "0, 0, 0" "1,1,1"))
      (Components|InstancedStaticMesh|AddInstance (Variables|Default|GetHISM_OvenKnob1) (Math|Transform|MakeTransform "15.500000,49.500000,84.500000" (Math|Rotator|MakeRotator 0.0 (* -1 (Variables|Default|GetRotate%20Knob%201)) 0.0) "1,1,1"))
      (Components|InstancedStaticMesh|AddInstance (Variables|Default|GetHISM_OvenKnob2) (Math|Transform|MakeTransform "26.250000,49.500000,84.500000" (Math|Rotator|MakeRotator 0.0 (* -1 (Variables|Default|GetRotate%20Knob%202)) 0.0) "1,1,1"))
      (Components|InstancedStaticMesh|AddInstance (Variables|Default|GetHISM_OvenKnob3) (Math|Transform|MakeTransform "37.000000,49.500000,84.500000" (Math|Rotator|MakeRotator 0.0 (* -1 (Variables|Default|GetRotate%20Knob%203)) 0.0) "1,1,1"))
      (Components|InstancedStaticMesh|AddInstance (Variables|Default|GetHISM_OvenKnob4) (Math|Transform|MakeTransform "47.750000,49.500000,84.500000" (Math|Rotator|MakeRotator 0.0 (* -1 (Variables|Default|GetRotate%20Knob%204)) 0.0) "1,1,1"))
      (Components|InstancedStaticMesh|AddInstance (Variables|Default|GetHISM_OvenKnob5) (Math|Transform|MakeTransform "58.500000,49.500000,84.500000" (Math|Rotator|MakeRotator 0.0 (* -1 (Variables|Default|GetRotate%20Knob%205)) 0.0) "1,1,1"))
      (Components|InstancedStaticMesh|AddInstance (Variables|Default|GetHISM_OvenHobs) (Math|Transform|MakeTransform "0, 0, 0" "0, 0, 0" "1,1,1")))
    (:then_1
      (if (Variables|Default|GetTray%20On/OFF)
        (Components|InstancedStaticMesh|AddInstance (Variables|Default|GetHISM_Tray) (Math|Transform|MakeTransform (Math|Vector|MakeVector 37.5 25.0 (+ (Variables|Default|GetAdjust%20Grille) 49.0)) "0, 0, 0" "1,1,1")))
      (if (Variables|Default|GetCountertop%20On/OFF)
        (Components|InstancedStaticMesh|AddInstance (Variables|Default|GetHISM_OvenCountertop) (Math|Transform|MakeTransform (Math|Vector|MakeVector 0.0 0.0 0.0) "0, 0, 0" "1,1,1")))
      (if (Variables|Default|GetFlame%20Front%20Left%20On/OFF)
        (Components|InstancedStaticMesh|AddInstance (Variables|Default|GetHISM_Flame_FrontLeft) (Math|Transform|MakeTransform (Math|Vector|MakeVector 0.0 0.0 0.0) "0, 0, 0" "1,1,1")))
      (if (Variables|Default|GetFlame%20Front%20Right%20On/OFF)
        (Components|InstancedStaticMesh|AddInstance (Variables|Default|GetHISM_Flame_FrontRight) (Math|Transform|MakeTransform (Math|Vector|MakeVector 0.0 0.0 0.0) "0, 0, 0" "1,1,1")))
      (if (Variables|Default|GetFlame%20Rear%20Left%20On/OFF)
        (Components|InstancedStaticMesh|AddInstance (Variables|Default|GetHISM_Flame_RearLeft) (Math|Transform|MakeTransform (Math|Vector|MakeVector 0.0 0.0 0.0) "0, 0, 0" "1,1,1")))
      (if (Variables|Default|GetFlame%20Rear%20Right%20On/OFF)
        (Components|InstancedStaticMesh|AddInstance (Variables|Default|GetHISM_Flame_RearRight) (Math|Transform|MakeTransform (Math|Vector|MakeVector 0.0 0.0 0.0) "0, 0, 0" "1,1,1"))))))