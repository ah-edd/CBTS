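; BP_Fridge is a configurable kitchen fridge prop with a fridge door and a freezer door, assembled in the construction script.
; It adds the main body and one door of each type as instances on hierarchical instanced static mesh components.
; SwapDoorAlignment picks left or right door meshes and flips hinge position and swing direction, while OpenFridge and OpenFreezer set each door's yaw.
; The event graph has no active logic.
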(event EventBeginPlay)

(event Collision|EventActorBeginOverlap
  (params (OtherActor :type Actor%20Object%20Reference)))

(event EventTick
  (params (DeltaSeconds :type Float%20%28single-precision%29)))

(fn ConstructionScript
  (bind _swap_door_alignment (Variables|Default|GetSwap%20Door%20Alignment))
  (bind _swap_door_alignment_2 (Variables|Default|GetSwap%20Door%20Alignment))
  (bind _swap_door_alignment_3 (Variables|Default|GetSwap%20Door%20Alignment))
  (Components|InstancedStaticMesh|AddInstance (Variables|Default|GetHISM_FridgeMain) (Math|Transform|MakeTransform "0, 0, 0" "0, 0, 0" "1,1,1"))
  (Components|InstancedStaticMesh|AddInstance (select _swap_door_alignment_3 (Variables|Default|GetHISM_FridgeDoor_R) (Variables|Default|GetHISM_FridgeDoor_L)) (Math|Transform|MakeTransform (Math|Vector|MakeVector (Math|Float|SelectFloat 7e+01 0.0 _swap_door_alignment) 5e+01 0.0) (Math|Rotator|MakeRotator 0.0 0.0 (* (Math|Float|SelectFloat -1.0 1.0 _swap_door_alignment) (Variables|Default|GetOpen%20Fridge))) "1,1,1"))
  (Components|InstancedStaticMesh|AddInstance (select _swap_door_alignment_3 (Variables|Default|GetHISM_FreezerDoor_R) (Variables|Default|GetHISM_FreezerDoor_L)) (Math|Transform|MakeTransform (Math|Vector|MakeVector (Math|Float|SelectFloat 7e+01 0.0 _swap_door_alignment_2) 5e+01 0.0) (Math|Rotator|MakeRotator 0.0 0.0 (* (Math|Float|SelectFloat -1.0 1.0 _swap_door_alignment_2) (Variables|Default|GetOpen%20Freezer))) "1,1,1")))