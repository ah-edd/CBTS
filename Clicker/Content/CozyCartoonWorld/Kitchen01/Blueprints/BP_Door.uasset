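; BP_Door is a configurable kitchen door prop that builds a frame and one door panel in its Construction Script.
; DoorSelection picks one of three panel styles, and SwapSide switches to the matching left-hand variant with a mirrored hinge position and swing.
; OpenDoor sets the panel's yaw, and both parts are added as Hierarchical Instanced Static Mesh instances.
; The event graph is empty, so the door has no runtime behavior.
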(event EventBeginPlay)

(event Collision|EventActorBeginOverlap
  (params (OtherActor :type Actor%20Object%20Reference)))

(event EventTick
  (params (DeltaSeconds :type Float%20%28single-precision%29)))

(fn ConstructionScript
  (bind _door_selection (Variables|Default|GetDoor%20Selection))
  (bind _open_door (Variables|Default|GetOpen%20Door))
  (Components|InstancedStaticMesh|AddInstance (Variables|Default|GetHISM_DoorFrame) (Math|Transform|MakeTransform "0, 0, 0" "0, 0, 0" "1,1,1"))
  (Components|InstancedStaticMesh|AddInstance (select (Variables|Default|GetSwap%20Side) (Utilities|Select :Index _door_selection :NewEnumerator1 (Variables|Default|GetHISM_Door_A_Left) :NewEnumerator2 (Variables|Default|GetHISM_Door_B_Left) :NewEnumerator0 (Variables|Default|GetHISM_Door_Plain_Left)) (Utilities|Select :Index _door_selection :NewEnumerator1 (Variables|Default|GetHISM_Door_A) :NewEnumerator2 (Variables|Default|GetHISM_Door_B) :NewEnumerator0 (Variables|Default|GetHISM_Door_Plain))) (Math|Transform|SelectTransform (Math|Transform|MakeTransform (Math|Vector|MakeVector 93.0 5.0 0.0) (Math|Rotator|MakeRotator 0.0 0.0 (* -1 _open_door)) "1,1,1") (Math|Transform|MakeTransform (Math|Vector|MakeVector 7.0 5.0 0.0) (Math|Rotator|MakeRotator 0.0 0.0 _open_door) "1,1,1") (Variables|Default|GetSwap%20Side))))