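; Modular kitchen cabinet prop that assembles itself from Hierarchical Instanced Static Mesh components in the construction script.
; It always adds one body, separator and left and right door instance, with door yaw set by per-side open variables and mirrored on the right.
; Boolean toggles add the countertop and each of the left and right shelves.
; It has no active runtime logic.
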(event EventBeginPlay)

(event Collision|EventActorBeginOverlap
  (params (OtherActor :type Actor%20Object%20Reference)))

(event EventTick
  (params (DeltaSeconds :type Float%20%28single-precision%29)))

(fn ConstructionScript
  (Utilities|FlowControl|Sequence
    (:then_0
      (Components|InstancedStaticMesh|AddInstance (Variables|Default|GetHISM_CabinetMain) (Math|Transform|MakeTransform "0, 0, 0" "0, 0, 0" "1,1,1"))
      (Components|InstancedStaticMesh|AddInstance (Variables|Default|GetHISM_CabinetSeparator) (Math|Transform|MakeTransform "0, 0, 0" "0, 0, 0" "1,1,1"))
      (Components|InstancedStaticMesh|AddInstance (Variables|Default|GetHISM_CabinetDoorLeft) (Math|Transform|MakeTransform "0, 0, 0" (Math|Rotator|MakeRotator 0.0 0.0 (Variables|Default|GetOpen%20Left%20Door)) "1,1,1"))
      (Components|InstancedStaticMesh|AddInstance (Variables|Default|GetHISM_CabinetDoorRight) (Math|Transform|MakeTransform "0, 0, 0" (Math|Rotator|MakeRotator 0.0 0.0 (* -1 (Variables|Default|GetOpen%20Right%20Door))) "1,1,1")))
    (:then_1
      (if (Variables|Default|GetCountertop%20On/Off)
        (Components|InstancedStaticMesh|AddInstance (Variables|Default|GetHISM_CabinetCountertop) (Math|Transform|MakeTransform "0, 0, 0" "0, 0, 0" "1,1,1")))
      (if (Variables|Default|GetLeft%20Shelf%20On/Off)
        (Components|InstancedStaticMesh|AddInstance (Variables|Default|GetHISM_CabinetShelfLeft) (Math|Transform|MakeTransform (Math|Vector|MakeVector 0.0 0.0 0.0) "0, 0, 0" "1,1,1")))
      (if (Variables|Default|GetRight%20Shelf%20On/Off)
        (Components|InstancedStaticMesh|AddInstance (Variables|Default|GetHISM_CabinetShelfRight) (Math|Transform|MakeTransform (Math|Vector|MakeVector 0.0 0.0 0.0) "0, 0, 0" "1,1,1"))))))