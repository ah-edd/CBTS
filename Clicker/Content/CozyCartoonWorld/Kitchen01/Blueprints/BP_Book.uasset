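; Kitchen prop Blueprint that procedurally builds either a single random book or a row of books in its Construction Script.
; A loop picks among three HISM book meshes, offsetting each instance by that book's width, with optional random count and side-switchable tilt.
; Random atlas materials get two random zone colors through dynamic material instances set on the HISM component, so color applies per book type rather than per instance.
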(event EventBeginPlay)

(event Collision|EventActorBeginOverlap
  (params (OtherActor :type Actor%20Object%20Reference)))

(event EventTick
  (params (DeltaSeconds :type Float%20%28single-precision%29)))

(fn ConstructionScript
  (bind _returnvalue (Math|Random|RandomFloatinRange 0.0 1.0))
  (bind _returnvalue_2 (Math|Random|RandomFloatinRange 0.0 1.0))
  (bind _returnvalue_3 (Math|Random|RandomFloatinRange 0.0 1.0))
  (bind _returnvalue_4 (Math|Random|RandomFloatinRange 0.0 1.0))
  (bind _returnvalue_5 (Math|Random|RandomFloatinRange 0.0 1.0))
  (bind _returnvalue_6 (Math|Random|RandomFloatinRange 0.0 1.0))
  (bind _number_of_different_types (Variables|Default|GetNumber%20of%20different%20types))
  (bind _book_rotation (Variables|Default|GetBook%20Rotation))
  (bind _switch_side (Variables|Default|GetSwitch%20Side))
  (bind _hism_booka (Variables|Default|GetHISM_BookA))
  (bind _hism_bookb (Variables|Default|GetHISM_BookB))
  (bind _hism_bookc (Variables|Default|GetHISM_BookC))
  (bind _returnvalue_7 (- _number_of_different_types 1))
  (bind _linearcolor (Utilities|Struct|MakeLinearColor _returnvalue _returnvalue_2 _returnvalue_3 1.0))
  (bind _linearcolor_2 (Utilities|Struct|MakeLinearColor _returnvalue_4 _returnvalue_5 _returnvalue_6 1.0))
  (bind _returnvalue_8 (Math|Random|RandomIntegerinRange 0 _returnvalue_7))
  (bind _returnvalue_9 (Utilities|Select :Index _returnvalue_8 :Option%200 _hism_booka :Option%201 _hism_bookb :Option%202 _hism_bookc))
  (if (Variables|Default|GetRow%20of%20Books)
    (LocalVariables|SetOffset%20Initial 0.0)
    (LocalVariables|SetOffset 0.0)
    (LocalVariables|SetBook%20Width 0.0)
    (for _index (range 0 (- (select (Variables|Default|GetRandom%20Number%20of%20Books) (Math|Random|RandomIntegerinRange (Variables|Default|GetRandom%20Number%20of%20Books%20MIN) (Variables|Default|GetRandom%20Number%20of%20Books%20MAX)) (Variables|Default|GetNumber%20of%20Books)) 1))
      (LocalVariables|SetRND (Math|Random|RandomIntegerinRange 0 (- (Variables|Default|GetNumber%20of%20different%20types) 1)))
      (if (== (Utilities|Select :Index (LocalVariables|GetRND) :Option%200 (Variables|Default|GetHISM_BookA) :Option%201 (Variables|Default|GetHISM_BookB) :Option%202 (Variables|Default|GetHISM_BookC)) "/Game/CozyCartoonWorld/Kitchen01/Meshes/SM_Book_A.SM_Book_A")
        (LocalVariables|SetBook%20Width 4.0)
        (elif (== (Utilities|Select :Index (LocalVariables|GetRND) :Option%200 (Variables|Default|GetHISM_BookA) :Option%201 (Variables|Default|GetHISM_BookB) :Option%202 (Variables|Default|GetHISM_BookC)) "/Game/CozyCartoonWorld/Kitchen01/Meshes/SM_Book_B.SM_Book_B")
          (LocalVariables|SetBook%20Width 5.0)
          (else
            (LocalVariables|SetBook%20Width 3.0))))
      (Utilities|FlowControl|Sequence
        (:then_0
          (Utilities|FlowControl|DoOnce false
            (:Completed
              (LocalVariables|SetOffset%20Initial (* -1 (LocalVariables|GetBook%20Width))))))
        (:then_1
          (Components|InstancedStaticMesh|AddInstance (Utilities|Select :Index (LocalVariables|GetRND) :Option%200 (Variables|Default|GetHISM_BookA) :Option%201 (Variables|Default|GetHISM_BookB) :Option%202 (Variables|Default|GetHISM_BookC)) (Math|Transform|MakeTransform (Math|Vector|MakeVector (+ (LocalVariables|GetOffset) (LocalVariables|GetBook%20Width) (LocalVariables|GetOffset%20Initial)) 0.0 (* _book_rotation (/ (Math|Float|SelectFloat 1.6 0.0 _switch_side) 25.0))) (Math|Rotator|MakeRotator 0.0 (Math|Float|SelectFloat (* -1 _book_rotation) _book_rotation _switch_side) 0.0) "1,1,1"))
          (LocalVariables|SetOffset (+ (LocalVariables|GetOffset) (LocalVariables|GetBook%20Width) (Utilities|Select :Index (LocalVariables|GetRND) :Option%200 1.0 :Option%201 2.0 :Option%202 0.0)))
          (bind _returnvalue_10 (Rendering|Material|CreateDynamicMaterialInstance (Utilities|Select :Index (LocalVariables|GetRND) :Option%200 (Variables|Default|GetHISM_BookA) :Option%201 (Variables|Default|GetHISM_BookB) :Option%202 (Variables|Default|GetHISM_BookC)) 0 (Utilities|Select :Index (Math|Random|RandomIntegerinRange 0 2) :Option%200 "/Game/CozyCartoonWorld/Kitchen01/Materials/Atlas/MI_Atlas_X_A1.MI_Atlas_X_A1" :Option%201 "/Game/CozyCartoonWorld/Kitchen01/Materials/Atlas/MI_Atlas_X_A2.MI_Atlas_X_A2" :Option%202 "/Game/CozyCartoonWorld/Kitchen01/Materials/Atlas/MI_Atlas_X_A3.MI_Atlas_X_A3") "None" :!class /Script/Engine.PrimitiveComponent))
          (Rendering|Material|SetVectorParameterValue _returnvalue_10 "Zone 1 Color" _linearcolor_2 :!class /Script/Engine.MaterialInstanceDynamic)
          (Rendering|Material|SetVectorParameterValue _returnvalue_10 "Zone 2 Color" _linearcolor_2 :!class /Script/Engine.MaterialInstanceDynamic))))
    (Utilities|FlowControl|DoOnce false) ; enters at Reset
    (else
      (Components|InstancedStaticMesh|AddInstance _returnvalue_9 (Math|Transform|MakeTransform (Math|Vector|MakeVector 0.0 0.0 0.0) "0, 0, 0" "1,1,1"))
      (bind _returnvalue_11 (Rendering|Material|CreateDynamicMaterialInstance _returnvalue_9 0 (Utilities|Select :Index (Math|Random|RandomIntegerinRange 0 2) :Option%200 "/Game/CozyCartoonWorld/Kitchen01/Materials/Atlas/MI_Atlas_X_A1.MI_Atlas_X_A1" :Option%201 "/Game/CozyCartoonWorld/Kitchen01/Materials/Atlas/MI_Atlas_X_A2.MI_Atlas_X_A2" :Option%202 "/Game/CozyCartoonWorld/Kitchen01/Materials/Atlas/MI_Atlas_X_A3.MI_Atlas_X_A3") "None" :!class /Script/Engine.PrimitiveComponent))
      (Rendering|Material|SetVectorParameterValue _returnvalue_11 "Zone 1 Color" _linearcolor :!class /Script/Engine.MaterialInstanceDynamic)
      (Rendering|Material|SetVectorParameterValue _returnvalue_11 "Zone 2 Color" _linearcolor :!class /Script/Engine.MaterialInstanceDynamic))))