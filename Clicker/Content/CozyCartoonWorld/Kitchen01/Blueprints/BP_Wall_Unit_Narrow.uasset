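; BP_Wall_Unit_Narrow is a configurable narrow kitchen wall cabinet prop, assembled in the construction script from instanced meshes.
; It adds the cabinet body, then a left door, either solid or glass-inset per GlassInsetDoorsSwap, with yaw set by OpenDoor.
; ShelfOnOff optionally adds a shelf instance.
; Each part uses its own HISM component, and the event graph has no active runtime logic.
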(event EventBeginPlay)

(event Collision|EventActorBeginOverlap
  (params (OtherActor :type Actor%20Object%20Reference)))

(event EventTick
  (params (DeltaSeconds :type Float%20%28single-precision%29)))

(fn ConstructionScript
  (Utilities|FlowControl|Sequence
    (:then_0
      (Components|InstancedStaticMesh|AddInstance (Variables|Default|GetHISM_CabinetMain) (Math|Transform|MakeTransform "0, 0, 0" "0, 0, 0" "1,1,1"))
      (Components|InstancedStaticMesh|AddInstance (select (Variables|Default|GetGlass%20Inset%20Doors%20Swap) (Variables|Default|GetHISM_CabinetDoorGlassLeft) (Variables|Default|GetHISM_CabinetDoorLeft)) (Math|Transform|MakeTransform "4.500000,32.000000, 0" (Math|Rotator|MakeRotator 0.0 0.0 (Variables|Default|GetOpen%20Door)) "1,1,1")))
    (:then_1
      (if (Variables|Default|GetShelf%20On/Off)
        (Components|InstancedStaticMesh|AddInstance (Variables|Default|GetHISM_CabinetShelf) (Math|Transform|MakeTransform (Math|Vector|MakeVector 0.0 0.0 0.0) "0, 0, 0" "1,1,1"))))))