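; BP_Microwave is a configurable kitchen microwave prop with an adjustable door and two knobs.
; The construction script adds one Hierarchical Instanced Static Mesh instance each for the body, door, upper knob and lower knob at fixed local offsets.
; The OpenDoor variable sets the door's yaw, while the negated RotateUpperKnob and RotateLowerKnob values set knob pitch.
; The event graph holds no runtime logic.
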(event EventBeginPlay)

(event Collision|EventActorBeginOverlap
  (params (OtherActor :type Actor%20Object%20Reference)))

(event EventTick
  (params (DeltaSeconds :type Float%20%28single-precision%29)))

(fn ConstructionScript
  (Components|InstancedStaticMesh|AddInstance (Variables|Default|GetHISM_MicrowaveMain) (Math|Transform|MakeTransform "0, 0, 0" "0, 0, 0" "1,1,1"))
  (Components|InstancedStaticMesh|AddInstance (Variables|Default|GetHISM_MicrowaveDoor) (Math|Transform|MakeTransform "-24.000000,14.500000,0.000000" (Math|Rotator|MakeRotator 0.0 0.0 (Variables|Default|GetOpen%20Door)) "1,1,1"))
  (Components|InstancedStaticMesh|AddInstance (Variables|Default|GetHISM_MicrowaveKnobUpper) (Math|Transform|MakeTransform "19.500000,16.750000,21.250000" (Math|Rotator|MakeRotator 0.0 (* -1 (Variables|Default|GetRotate%20Upper%20Knob)) 0.0) "1,1,1"))
  (Components|InstancedStaticMesh|AddInstance (Variables|Default|GetHISM_MicrowaveKnobLower) (Math|Transform|MakeTransform "19.500000,16.750000,14.000000" (Math|Rotator|MakeRotator 0.0 (* -1 (Variables|Default|GetRotate%20Lower%20Knob)) 0.0) "1,1,1")))