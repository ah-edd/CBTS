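; Construction-time prop blueprint for a tall kitchen wall cabinet in the Cozy Cartoon World kitchen set.
; The construction script adds single instances to hierarchical instanced static mesh components for the body, shelf and left and right glass doors.
; OpenLeftDoor and OpenRightDoor set each door's yaw, with the right negated so the doors mirror when opened.
; It has no runtime logic.
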(event EventBeginPlay)

(event Collision|EventActorBeginOverlap
  (params (OtherActor :type Actor%20Object%20Reference)))

(event EventTick
  (params (DeltaSeconds :type Float%20%28single-precision%29)))

(fn ConstructionScript
  (Components|InstancedStaticMesh|AddInstance (Variables|Default|GetHISM_CabinetMain) (Math|Transform|MakeTransform "0, 0, 0" "0, 0, 0" "1,1,1"))
  (Components|InstancedStaticMesh|AddInstance (Variables|Default|GetHISM_CabinetShelf) (Math|Transform|MakeTransform (Math|Vector|MakeVector 0.0 0.0 0.0) "0, 0, 0" "1,1,1"))
  (Components|InstancedStaticMesh|AddInstance (Variables|Default|GetHISM_CabinetDoorGlassLeft) (Math|Transform|MakeTransform "4.500000,32.000000, 0" (Math|Rotator|MakeRotator 0.0 0.0 (Variables|Default|GetOpen%20Left%20Door)) "1,1,1"))
  (Components|InstancedStaticMesh|AddInstance (Variables|Default|GetHISM_CabinetDoorGlassRight) (Math|Transform|MakeTransform "95.250000,32.000000, 0" (Math|Rotator|MakeRotator 0.0 0.0 (* -1 (Variables|Default|GetOpen%20Right%20Door))) "1,1,1")))