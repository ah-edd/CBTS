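; Narrow kitchen cabinet prop Blueprint, assembled in the Construction Script from hierarchical instanced static mesh components.
; It adds one instance each for the body and the top, middle and bottom drawers, with per-drawer variables setting each drawer's Y offset to pose it open.
; A toggle optionally adds a countertop instance.
; The event graph is empty, so there is no runtime behavior.
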(event EventBeginPlay)

(event Collision|EventActorBeginOverlap
  (params (OtherActor :type Actor%20Object%20Reference)))

(event EventTick
  (params (DeltaSeconds :type Float%20%28single-precision%29)))

(fn ConstructionScript
  (Utilities|FlowControl|Sequence
    (:then_0
      (Components|InstancedStaticMesh|AddInstance (Variables|Default|GetHISM_CabinetMain) (Math|Transform|MakeTransform "0, 0, 0" "0, 0, 0" "1,1,1"))
      (Components|InstancedStaticMesh|AddInstance (Variables|Default|GetHISM_CabinetDrawerBottom) (Math|Transform|MakeTransform (Math|Vector|MakeVector 0.0 (Variables|Default|GetOpen%20Bottom%20Drawer) 0.0) "0, 0, 0" "1,1,1"))
      (Components|InstancedStaticMesh|AddInstance (Variables|Default|GetHISM_CabinetDrawerMid) (Math|Transform|MakeTransform (Math|Vector|MakeVector 0.0 (Variables|Default|GetOpen%20Middle%20Drawer) 0.0) "0, 0, 0" "1,1,1"))
      (Components|InstancedStaticMesh|AddInstance (Variables|Default|GetHISM_CabinetDrawerTop) (Math|Transform|MakeTransform (Math|Vector|MakeVector 0.0 (Variables|Default|GetOpen%20Top%20Drawer) 0.0) "0, 0, 0" "1,1,1")))
    (:then_1
      (if (Variables|Default|GetCountertop%20On/Off)
        (Components|InstancedStaticMesh|AddInstance (Variables|Default|GetHISM_CabinetCountertop) (Math|Transform|MakeTransform "0, 0, 0" "0, 0, 0" "1,1,1"))))))