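; Tumble dryer prop for the CozyCartoonWorld kitchen set, posed through variables rather than animated at runtime.
; The construction script assembles it from separate hierarchical instanced static mesh components for body, door, drum and knob, each placed at a fixed offset.
; Variables set door yaw, drum pitch and negated knob pitch, and a boolean adds an optional countertop.
; The event graph holds no active logic.
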(event EventBeginPlay)

(event Collision|EventActorBeginOverlap
  (params (OtherActor :type Actor%20Object%20Reference)))

(event EventTick
  (params (DeltaSeconds :type Float%20%28single-precision%29)))

(fn ConstructionScript
  (Components|InstancedStaticMesh|AddInstance (Variables|Default|GetHISM_TumbleDryerMain) (Math|Transform|MakeTransform "0, 0, 0" "0, 0, 0" "1,1,1"))
  (Components|InstancedStaticMesh|AddInstance (Variables|Default|GetHISM_TumbleDryerDoor) (Math|Transform|MakeTransform "9.500000,48.000000,0.000000" (Math|Rotator|MakeRotator 0.0 0.0 (Variables|Default|GetOpen%20Door)) "1,1,1"))
  (Components|InstancedStaticMesh|AddInstance (Variables|Default|GetHISM_TumbleDryerDrum) (Math|Transform|MakeTransform "37.500000,10.000000,48.400002" (Math|Rotator|MakeRotator 0.0 (Variables|Default|GetRotate%20Drum) 0.0) "1,1,1"))
  (Components|InstancedStaticMesh|AddInstance (Variables|Default|GetHISM_TumbleDryerKnob) (Math|Transform|MakeTransform "55.500000,49.500000,86.000000" (Math|Rotator|MakeRotator 0.0 (* -1 (Variables|Default|GetRotate%20Knob)) 0.0) "1,1,1"))
  (if (Variables|Default|GetCountertop%20On/Off)
    (Components|InstancedStaticMesh|AddInstance (Variables|Default|GetHISM_TumbleDryerCountertop) (Math|Transform|MakeTransform "0, 0, 0" "0, 0, 0" "1,1,1"))))