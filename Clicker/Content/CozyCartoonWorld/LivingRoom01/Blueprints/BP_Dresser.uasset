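; BP_Dresser is a configurable dresser furniture prop in the Cozy Cartoon World living room set.
; The construction script adds a main body instance, then optional shelves, doors and three drawers, each to its own HISM component.
; Variables toggle each part and set shelf heights, mirrored door swing angles, drawer pull-out distances and whether drawers sit on the left.
; The event graph holds no runtime logic.
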(event EventBeginPlay)

(event Collision|EventActorBeginOverlap
  (params (OtherActor :type Actor%20Object%20Reference)))

(event EventTick
  (params (DeltaSeconds :type Float%20%28single-precision%29)))

(fn ConstructionScript
  (bind _drawers_on_left (Variables|Default|GetDrawers%20on%20Left))
  (bind _returnvalue (Math|Float|SelectFloat -45.25 0.0 _drawers_on_left))
  (Components|InstancedStaticMesh|AddInstance (Variables|Default|GetHISM_DresserMain) (Math|Transform|MakeTransform "0, 0, 0" "0, 0, 0" "1,1,1"))
  (Utilities|FlowControl|Sequence
    (:then_0
      (if (Variables|Default|GetLeft%20Shelf)
        (Components|InstancedStaticMesh|AddInstance (Variables|Default|GetHISM_DresserShelfLeft) (Math|Transform|MakeTransform (Math|Vector|MakeVector 0.0 0.0 (Variables|Default|GetLeft%20Shelf%20Position)) "0, 0, 0" "1,1,1"))))
    (:then_1
      (if (Variables|Default|GetRight%20Shelf)
        (Components|InstancedStaticMesh|AddInstance (Variables|Default|GetHISM_DresserShelfRight) (Math|Transform|MakeTransform (Math|Vector|MakeVector 0.0 0.0 (Variables|Default|GetRight%20Shelf%20Position)) "0, 0, 0" "1,1,1"))))
    (:then_2
      (if (Variables|Default|GetLeft%20Door)
        (Components|InstancedStaticMesh|AddInstance (Variables|Default|GetHISM_DresserDoorfLeft) (Math|Transform|MakeTransform "-42.250000,38.000000,11.500000" (Math|Rotator|MakeRotator 0.0 0.0 (Variables|Default|GetOpen%20Left%20Door)) "1,1,1"))))
    (:then_3
      (if (Variables|Default|GetRight%20Door)
        (Components|InstancedStaticMesh|AddInstance (Variables|Default|GetHISM_DresserDoorRight) (Math|Transform|MakeTransform "42.250000,38.000000,11.500000" (Math|Rotator|MakeRotator 0.0 0.0 (* -1 (Variables|Default|GetOpen%20Right%20Door))) "1,1,1"))))
    (:then_4
      (Utilities|FlowControl|Sequence
        (:then_0
          (if (Variables|Default|GetTop%20Drawer)
            (Components|InstancedStaticMesh|AddInstance (Variables|Default|GetHISM_DresserDrawerTop) (Math|Transform|MakeTransform (Math|Vector|MakeVector _returnvalue (Variables|Default|GetOpen%20Top%20Drawer) 0.0) "0, 0, 0" "1,1,1"))))
        (:then_1
          (if (Variables|Default|GetMid%20Drawer)
            (Components|InstancedStaticMesh|AddInstance (Variables|Default|GetHISM_DresserDrawerMid) (Math|Transform|MakeTransform (Math|Vector|MakeVector _returnvalue (Variables|Default|GetOpen%20Mid%20Drawer) 0.0) "0, 0, 0" "1,1,1"))))
        (:then_2
          (if (Variables|Default|GetBottom%20Drawer)
            (Components|InstancedStaticMesh|AddInstance (Variables|Default|GetHISM_DresserDrawerBottom) (Math|Transform|MakeTransform (Math|Vector|MakeVector _returnvalue (Variables|Default|GetOpen%20Bottom%20Drawer) 0.0) "0, 0, 0" "1,1,1"))))))))