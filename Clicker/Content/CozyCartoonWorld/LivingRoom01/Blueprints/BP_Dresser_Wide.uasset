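; BP_Dresser_Wide is a wide dresser prop with top, middle and bottom drawers whose open positions are adjustable.
; The construction script adds one instance each to separate hierarchical instanced static mesh components for the body and the three drawers.
; Each drawer's Y offset comes from its own open variable, so the pose is set at construction.
; It has no runtime logic; the event graph holds only disabled placeholder events.
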(event EventBeginPlay)

(event Collision|EventActorBeginOverlap
  (params (OtherActor :type Actor%20Object%20Reference)))

(event EventTick
  (params (DeltaSeconds :type Float%20%28single-precision%29)))

(fn ConstructionScript
  (Components|InstancedStaticMesh|AddInstance (Variables|Default|GetHISM_DresserMain) (Math|Transform|MakeTransform "0, 0, 0" "0, 0, 0" "1,1,1"))
  (Utilities|FlowControl|Sequence
    (:then_0
      (Components|InstancedStaticMesh|AddInstance (Variables|Default|GetHISM_DresserDrawerTop) (Math|Transform|MakeTransform (Math|Vector|MakeVector 0.0 (Variables|Default|GetOpen%20Top%20Drawer) 0.0) "0, 0, 0" "1,1,1")))
    (:then_1
      (Components|InstancedStaticMesh|AddInstance (Variables|Default|GetHISM_DresserDrawerMid) (Math|Transform|MakeTransform (Math|Vector|MakeVector 0.0 (Variables|Default|GetOpen%20Mid%20Drawer) 0.0) "0, 0, 0" "1,1,1")))
    (:then_2
      (Components|InstancedStaticMesh|AddInstance (Variables|Default|GetHISM_DresserDrawerBottom) (Math|Transform|MakeTransform (Math|Vector|MakeVector 0.0 (Variables|Default|GetOpen%20Bottom%20Drawer) 0.0) "0, 0, 0" "1,1,1")))))