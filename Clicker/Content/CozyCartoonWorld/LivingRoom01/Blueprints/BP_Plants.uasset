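; Configurable potted plant prop for the living room set, assembled in the construction script from a chosen pot or vase and a chosen plant.
; The selected container gets an instance at the origin of its hierarchical instanced mesh component.
; The container's row in DT_Plants then supplies a vector for the selected plant, with X setting its height and Y its uniform scale.
; The event graph holds no logic.
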(event EventBeginPlay)

(event Collision|EventActorBeginOverlap
  (params (OtherActor :type Actor%20Object%20Reference)))

(event EventTick
  (params (DeltaSeconds :type Float%20%28single-precision%29)))

(fn ConstructionScript
  (bind _plant_selection (Variables|Default|GetPlant%20Selection))
  (bind _vase_pot_selection (Variables|Default|GetVase/Pot%20Selection))
  (Components|InstancedStaticMesh|AddInstance (Utilities|Select :Index _vase_pot_selection :NewEnumerator0 (Variables|Default|GetHISM_Flowerpot_Large_A) :NewEnumerator1 (Variables|Default|GetHISM_Flowerpot_Large_B) :NewEnumerator2 (Variables|Default|GetHISM_Flowerpot_Small_A) :NewEnumerator3 (Variables|Default|GetHISM_Flowerpot_Small_B) :NewEnumerator4 (Variables|Default|GetHISM_Flowerpot_Vase_A) :NewEnumerator5 (Variables|Default|GetHISM_Flowerpot_Vase_B) :NewEnumerator6 (Variables|Default|GetHISM_Flowerpot_Vase_C) :NewEnumerator7 (Variables|Default|GetHISM_Flowerpot_Vase_D) :NewEnumerator8 (Variables|Default|GetHISM_Flowerpot_Floor_Vase)) (Math|Transform|MakeTransform "0, 0, 0" "0, 0, 0" "1,1,1"))
  (bind _returnvalue (Utilities|GetDataTableRow "/Game/CozyCartoonWorld/LivingRoom01/Blueprints/DT_Plants.DT_Plants" (Utilities|Select :Index _vase_pot_selection :NewEnumerator0 "FlowerpotLargeA" :NewEnumerator1 "FlowerpotLargeB" :NewEnumerator2 "FlowerpotSmallA" :NewEnumerator3 "FlowerpotSmallB" :NewEnumerator4 "VaseA" :NewEnumerator5 "VaseB" :NewEnumerator6 "VaseC" :NewEnumerator7 "VaseD" :NewEnumerator8 "FloorVase"))
    (:then
      (Components|InstancedStaticMesh|AddInstance (Utilities|Select :Index _plant_selection :NewEnumerator0 (Variables|Default|GetHISM_Plant_A) :NewEnumerator1 (Variables|Default|GetHISM_Plant_B) :NewEnumerator2 (Variables|Default|GetHISM_Snake_Plant) :NewEnumerator3 (Variables|Default|GetHISM_Flower_A) :NewEnumerator4 (Variables|Default|GetHISM_Flower_B)) (Math|Transform|MakeTransform (Math|Vector|MakeVector 0.0 0.0 (.x (Utilities|Select :Index _plant_selection :NewEnumerator0 (.PlantA (Utilities|Struct|BreakST_Plants _returnvalue)) :NewEnumerator1 (.PlantB (Utilities|Struct|BreakST_Plants _returnvalue)) :NewEnumerator2 (.SnakePlant (Utilities|Struct|BreakST_Plants _returnvalue)) :NewEnumerator3 (.FlowerA (Utilities|Struct|BreakST_Plants _returnvalue)) :NewEnumerator4 (.FlowerB (Utilities|Struct|BreakST_Plants _returnvalue))))) "0, 0, 0" (Math|Vector|MakeVector (.y (Utilities|Select :Index _plant_selection :NewEnumerator0 (.PlantA (Utilities|Struct|BreakST_Plants _returnvalue)) :NewEnumerator1 (.PlantB (Utilities|Struct|BreakST_Plants _returnvalue)) :NewEnumerator2 (.SnakePlant (Utilities|Struct|BreakST_Plants _returnvalue)) :NewEnumerator3 (.FlowerA (Utilities|Struct|BreakST_Plants _returnvalue)) :NewEnumerator4 (.FlowerB (Utilities|Struct|BreakST_Plants _returnvalue)))) (.y (Utilities|Select :Index _plant_selection :NewEnumerator0 (.PlantA (Utilities|Struct|BreakST_Plants _returnvalue)) :NewEnumerator1 (.PlantB (Utilities|Struct|BreakST_Plants _returnvalue)) :NewEnumerator2 (.SnakePlant (Utilities|Struct|BreakST_Plants _returnvalue)) :NewEnumerator3 (.FlowerA (Utilities|Struct|BreakST_Plants _returnvalue)) :NewEnumerator4 (.FlowerB (Utilities|Struct|BreakST_Plants _returnvalue)))) (.y (Utilities|Select :Index _plant_selection :NewEnumerator0 (.PlantA (Utilities|Struct|BreakST_Plants _returnvalue)) :NewEnumerator1 (.PlantB (Utilities|Struct|BreakST_Plants _returnvalue)) :NewEnumerator2 (.SnakePlant (Utilities|Struct|BreakST_Plants _returnvalue)) :NewEnumerator3 (.FlowerA (Utilities|Struct|BreakST_Plants _returnvalue)) :NewEnumerator4 (.FlowerB (Utilities|Struct|BreakST_Plants _returnvalue))))))))))