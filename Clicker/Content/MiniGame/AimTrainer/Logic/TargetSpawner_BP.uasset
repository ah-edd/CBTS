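; Gridshot target spawner for the aim trainer minigame, keeping up to five BP_GridshotTarget actors alive in a box volume.
; BeginPlay fills the volume, then a fast looping timer counts live targets and spawns replacements below the cap.
; Each spawns at a random point in the Spawnarea box, turned toward the player camera with a 90-degree yaw offset.
; The construction script sizes the box from an extent variable.
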(event Custom|Spawn%20Target
  (bind _spawnarea (Variables|Default|Getspawnarea))
  (bind _outactors (Actor|GetAllActorsOfClass "/Game/AimTrainer/BP_GridshotTarget.BP_GridshotTarget_C"))
  (if (<= (Utilities|Array|Length _outactors) 4)
    (bind _output_get (Variables|Default|Setspawmlocation (Math|Random|RandomPointinBoundingBox (Transformation|GetWorldLocation _spawnarea) (Components|Box|GetScaledBoxExtent _spawnarea))))
    (Game|SpawnActorfromClass "/Game/AimTrainer/BP_GridshotTarget.BP_GridshotTarget_C" (Math|Transform|MakeTransform _output_get (Math|Rotator|MakeRotator (.roll (Math|Rotator|FindLookatRotation _output_get (Transformation|GetWorldLocation (Variables|/Script/Engine.PlayerCameraManager|GetTransformComponent (Game|GetPlayerCameraManager 0))))) (.pitch (Math|Rotator|FindLookatRotation _output_get (Transformation|GetWorldLocation (Variables|/Script/Engine.PlayerCameraManager|GetTransformComponent (Game|GetPlayerCameraManager 0))))) (+ (.yaw (Math|Rotator|FindLookatRotation _output_get (Transformation|GetWorldLocation (Variables|/Script/Engine.PlayerCameraManager|GetTransformComponent (Game|GetPlayerCameraManager 0))))) 9e+01)) "1.000000,1.000000,1.000000") "AdjustIfPossibleButAlwaysSpawn" "MultiplyWithRoot" 0 "0.000000,0.000000,0.000000" 0)))

(event EventBeginPlay
  (Utilities|Time|SetTimerbyEvent (delegate Custom|Spawn%20Target) 0.02 true)
  (for _index (range 0 5)
    (CallFunction|SpawnTarget)))

(fn ConstructionScript
  (Components|Box|SetBoxExtent (Variables|Default|Getspawnarea) (Variables|Default|GetIn%20Box%20Extent) true))