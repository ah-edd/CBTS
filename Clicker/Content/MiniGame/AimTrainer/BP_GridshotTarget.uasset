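; BP_GridshotTarget is a shootable target for the Gridshot aim trainer minigame.
; When damaged, it plays a pop sound, asks BP_GridshotBox to spawn a target by passing a location, adds points to the player's BP_MenuCharacter, then destroys itself.
; Leftover movement logic for drifting the sphere toward random points in a box is disconnected and never runs.
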(event Custom|MoveTarget
  ;[1 1 1] This is seperate movement logic, pls ignore sorry
)

(event EventBeginPlay
  ;[1 1 1] This is seperate movement logic, pls ignore sorry
)

(event Collision|EventActorBeginOverlap
  (params (OtherActor :type Actor%20Object%20Reference)))

(event EventTick
  (params (DeltaSeconds :type Float%20%28single-precision%29))
  ;[1 1 1] This is seperate movement logic, pls ignore sorry
)

(event Game|Damage|EventAnyDamage
  (params (Damage :type Float%20%28single-precision%29) (DamageType :type Damage%20Type%20Object%20Reference) (InstigatedBy :type Controller%20Object%20Reference) (DamageCauser :type Actor%20Object%20Reference))
  (bind _returnvalue (Game|GetPlayerCharacter 0))
  (bind _asbp_menu_character (Utilities|Casting|CastToBP_MenuCharacter _returnvalue))
  ;[1 1 1] On hit adds points
  (Audio|PlaySound2D "/Game/Sound/happy-pop-2-185287__1_.happy-pop-2-185287__1_" 1.0 1.0 0.0 0 0)
  (bind _returnvalue_2 (Actor|GetActorOfClass "/Game/MiniGame/AimTrainer/BP_GridshotBox.BP_GridshotBox_C"))
  (Default|SpawnTarget _returnvalue_2 (Variables|Default|GetLocation))
  (Variables|/Game/Blueprints/BP_MenuCharacter.BP_MenuCharacter_C|SetPoints _asbp_menu_character (+ (Variables|/Game/Blueprints/BP_MenuCharacter.BP_MenuCharacter_C|GetPoints _asbp_menu_character) 10))
  (Actor|DestroyActor))

(fn ConstructionScript)