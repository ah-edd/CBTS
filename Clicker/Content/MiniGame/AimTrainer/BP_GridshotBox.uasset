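; Spawn area for a Gridshot aim-trainer minigame that keeps targets on random points of a grid.
; The construction script builds the point grid from Y/Z scale and spacing, and fits a box component to it.
; When BP_Menu is destroyed, five targets spawn, each point leaving the free pool.
; SpawnTarget spawns a replacement before returning the passed location to the pool, avoiding immediate reuse.
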(event OnDestroyedDispatch(InstructionsReference))

(event Custom|Spawn%20Target
  (params (Location :type Vector))
  (bind _unactivespawnpoints (Variables|Default|GetUnactiveSpawnPoints))
  (bind _activespawnpoints (Variables|Default|GetActiveSpawnPoints))
  (Variables|Default|SetLatestLocation Location)
  (bind _returnvalue (Utilities|Array|Add _unactivespawnpoints (.OutItem (Utilities|Array|Random _activespawnpoints))))
  (Utilities|Array|RemoveItem _activespawnpoints (Utilities|Array|Get(acopy) _unactivespawnpoints _returnvalue))
  (Game|SpawnActorfromClass "/Game/MiniGame/AimTrainer/BP_GridshotTarget.BP_GridshotTarget_C" (Math|Transform|MakeTransform (Math|Transform|TransformLocation (Transformation|GetActorTransform) (Utilities|Array|Get(acopy) _unactivespawnpoints _returnvalue)) "0, 0, 0" "0.250000,0.250000,0.250000") "AlwaysSpawn" "MultiplyWithRoot" 0 (Utilities|Array|Get(acopy) _unactivespawnpoints _returnvalue) 0)
  (if (Variables|Default|GetActive)
    (Utilities|Array|RemoveItem (Variables|Default|GetUnactiveSpawnPoints) (Variables|Default|GetLatestLocation))
    (Utilities|Array|Add (Variables|Default|GetActiveSpawnPoints) (Variables|Default|GetLatestLocation))))

(event Custom|StartTargets
  (bind _unactivespawnpoints (Variables|Default|GetUnactiveSpawnPoints))
  (bind _latestlocation (Variables|Default|GetLatestLocation))
  (bind _activespawnpoints (Variables|Default|GetActiveSpawnPoints))
  (for _index (range 1 5)
    (bind _returnvalue (Utilities|Array|Add _unactivespawnpoints (.OutItem (Utilities|Array|Random _activespawnpoints))))
    (Utilities|Array|RemoveItem _activespawnpoints (Utilities|Array|Get(acopy) _unactivespawnpoints _returnvalue))
    (Game|SpawnActorfromClass "/Game/MiniGame/AimTrainer/BP_GridshotTarget.BP_GridshotTarget_C" (Math|Transform|MakeTransform (Math|Transform|TransformLocation (Transformation|GetActorTransform) (Utilities|Array|Get(acopy) _unactivespawnpoints _returnvalue)) "0, 0, 0" "0.250000,0.250000,0.250000") "AlwaysSpawn" "MultiplyWithRoot" 0 (Utilities|Array|Get(acopy) _unactivespawnpoints _returnvalue) 0)
    (if (Variables|Default|GetActive)
      (Utilities|Array|RemoveItem (Variables|Default|GetUnactiveSpawnPoints) _latestlocation)
      (Utilities|Array|Add (Variables|Default|GetActiveSpawnPoints) _latestlocation)))
  (Variables|Default|SetActive true))

(event Custom|aaa
  (CallFunction|StartTargets))

(event EventBeginPlay
  (bind _returnvalue (Actor|GetActorOfClass "/Game/Blueprints/BP_Menu.BP_Menu_C"))
  (EventDispatchers|BindEventtoOnDestroyedDispatch _returnvalue (delegate Custom|aaa)))

(fn ConstructionScript
  (bind _spacing (Variables|Default|GetSpacing))
  (bind _spacing_2 (Variables|Default|GetSpacing))
  (bind _box (Variables|Default|GetBox))
  (bind _returnvalue (/ _spacing_2 1e+02))
  (for _index (range 1 (Variables|Default|GetYScale))
    (for _index_2 (range 1 (Variables|Default|GetZScale))
      (Utilities|Array|Add (Variables|Default|GetActiveSpawnPoints) (Math|Vector|MakeVector 0.0 (* (- _index 1) _spacing) (* (- _index_2 1) _spacing)))
      (Components|Box|SetBoxExtent _box (Math|Vector|MakeVector 1.0 (* (Math|Conversions|ToFloat(Integer) (Variables|Default|GetYScale)) _returnvalue) (* (Math|Conversions|ToFloat(Integer) (Variables|Default|GetZScale)) _returnvalue)) true)
      (Transformation|SetRelativeLocation _box (* (Variables|/Script/Engine.BoxComponent|GetBoxExtent (Variables|Default|GetBox)) 2e+01) false false))))