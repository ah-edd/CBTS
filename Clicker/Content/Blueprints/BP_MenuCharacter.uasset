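; BP_MenuCharacter is a first-person-style character with mouse look and click-to-shoot line tracing.
; Look axes feed controller yaw and pitch, and left click traces from the camera on Visibility, prints the hit component and applies point damage.
; BeginPlay creates two WB_GameUI widgets, showing one and storing the other as InteractWidget.
; An interaction trace using that widget is unfinished and never runs.
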(event EventBeginPlay
  (bind _returnvalue (UserInterface|CreateWidget "/Game/Widgets/WB_GameUI.WB_GameUI_C"))
  (UserInterface|Viewport|AddtoViewport _returnvalue 0)
  (bind _returnvalue_2 (UserInterface|CreateWidget "/Game/Widgets/WB_GameUI.WB_GameUI_C"))
  (Variables|Default|SetInteract%20Widget _returnvalue_2))

(event Collision|EventActorBeginOverlap
  (params (OtherActor :type Actor%20Object%20Reference)))

(event Input|AxisEvents|InputAxisLookX
  (params (AxisValue :type Float%20%28single-precision%29))
  (Pawn|Input|AddControllerYawInput (Game|GetPlayerCharacter 0) AxisValue))

(event Input|AxisEvents|InputAxisLookY
  (params (AxisValue :type Float%20%28single-precision%29))
  (Pawn|Input|AddControllerPitchInput (Game|GetPlayerCharacter 0) AxisValue))

(event Input|MouseEvents|LeftMouseButton
  (params (Key :type Key%20Structure :default "None"))
  (bind _camera (Variables|Default|GetCamera))
  (bind _returnvalue (Transformation|GetWorldLocation _camera))
  (:Pressed
    (Utilities|FlowControl|Sequence
      (:then_0
        (bind _outhit (Collision|LineTraceByChannel _returnvalue (+ (* (Math|Vector|GetForwardVector (Transformation|GetWorldRotation _camera)) (Variables|Default|GetTraceDistance)) _returnvalue) "TraceTypeQuery1" false 0 "None"))
        (Development|PrintString (Utilities|GetDisplayName (.HitComponent (Collision|BreakHitResult _outhit))))
        (Game|Damage|ApplyPointDamage (.HitActor (Collision|BreakHitResult _outhit)) 1e+02 (Transformation|GetActorLocation (Game|GetPlayerCharacter 0)) _outhit)))))

(fn ConstructionScript)