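; BP_Menu is a menu actor that acts as a destructible play button.
; Point damage is ignored until a five-second delay after BeginPlay, then any hit zeroes PlayButtonHealth and issues an ApplyPointDamage call.
; Tick polls that health and, at zero, enables tilting on the player's BP_MenuCharacter, plays a retro sound, destroys the actor and fires its OnDestroyed dispatcher.
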(event EventBeginPlay
  (Utilities|FlowControl|Delay 5.0)
  (Variables|Default|SetCanBeDestroyed true))

(event Collision|EventActorBeginOverlap
  (params (OtherActor :type Actor%20Object%20Reference)))

(event EventTick
  (params (DeltaSeconds :type Float%20%28single-precision%29))
  (if (<= (Variables|Default|GetPlayButtonHealth) 0.0)
    (Variables|Default|SetIsDestroyed true)
    (bind _asbp_menu_character (Utilities|Casting|CastToBP_MenuCharacter (Game|GetPlayerCharacter 0)))
    (Variables|/Game/Blueprints/BP_MenuCharacter.BP_MenuCharacter_C|SetCanTilt? _asbp_menu_character true)
    (Audio|PlaySound2D "/Game/MiniGame/AimTrainer/SoundFX/Sounds/Retro10.Retro10" 1.0 1.0 0.0 0 0)
    (Actor|DestroyActor)
    (Default|CallOnDestroyedDispatch)))

(event Game|Damage|EventPointDamage
  (params (Damage :type Float%20%28single-precision%29) (DamageType :type Damage%20Type%20Object%20Reference) (HitLocation :type Vector :default "0, 0, 0") (HitNormal :type Vector :default "0, 0, 0") (HitComponent :type Primitive%20Component%20Object%20Reference) (BoneName :type Name :default "None") (ShotFromDirection :type Vector :default "0, 0, 0") (InstigatedBy :type Controller%20Object%20Reference) (DamageCauser :type Actor%20Object%20Reference) (HitInfo :type Hit%20Result%20Structure%20%28by%20ref%29))
  (if (Variables|Default|GetCanBeDestroyed)
    (Variables|Default|SetPlayButtonHealth 0.0)
    (Game|Damage|ApplyPointDamage 0 1e+02 HitLocation (Collision|MakeHitResult true true 0.0 0.0 "0, 0, 0" "0, 0, 0" "0,0,1" "0,0,1" 0 0 (Variables|Default|GetBox)))))

(fn ConstructionScript)